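; BP_WorldDoorInverse is a world door that swings open on overlap, with the swing direction set by the side of approach.
; FrontCheck and BackCheck overlaps set opposite direction signs, which multiply a timeline curve driving the Door's relative yaw.
; Leaving CloseCheck reverses the timeline from its end, with IsDoorOpening guarding against retriggers.
; Overlaps do not filter by actor, and opening and closing print debug strings.
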(event `self.FrontCheck.OnComponentBeginOverlap`
  (params (OverlappedComponent :type "PrimitiveComponent Object Reference") (OtherActor :type "Actor Object Reference") (OtherComp :type "PrimitiveComponent Object Reference") (OtherBodyIndex :type Integer) (bFromSweep :type Boolean) (SweepResult :type "HitResult Structure (by ref)"))
  (if (not (`self.IsDoorOpening`))
    (set `self.OpenDirection` -1.0)
    (set `self.IsDoorOpening` true :!label _label)
    (`KismetSystemLibrary.PrintString` "Open")
    (bind (_direction _doorrotationz) (`Timeline|DoorTimelineComponent` :!via `PlayFromStart` :!label _label_2)
      (:`Update`
        (`SceneComponent.K2_SetRelativeRotation` (`self.Door`) (`KismetMathLibrary.MakeRotator` 0.0 0.0 (* _doorrotationz (`self.OpenDirection`))) false false)))))

(event `self.BackCheck.OnComponentBeginOverlap`
  (params (OverlappedComponent :type "PrimitiveComponent Object Reference") (OtherActor :type "Actor Object Reference") (OtherComp :type "PrimitiveComponent Object Reference") (OtherBodyIndex :type Integer) (bFromSweep :type Boolean) (SweepResult :type "HitResult Structure (by ref)"))
  (if (not (`self.IsDoorOpening`))
    (set `self.OpenDirection` 1.0)
    (goto _label)))

(event `self.CloseCheck.OnComponentEndOverlap`
  (params (OverlappedComponent :type "PrimitiveComponent Object Reference") (OtherActor :type "Actor Object Reference") (OtherComp :type "PrimitiveComponent Object Reference") (OtherBodyIndex :type Integer))
  (if (`self.IsDoorOpening`)
    (`KismetSystemLibrary.PrintString` "Close")
    (set `self.IsDoorOpening` false)
    (goto _label_2 :!via `ReverseFromEnd`)))

(fn `UserConstructionScript`)