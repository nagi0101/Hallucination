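; Test enemy AI that reacts to sounds through AI Perception hearing and feeds its Blackboard.
; BeginPlay seeds the keys, then each heard stimulus writes location, distance, volume and a heard flag.
; It stores the first sound location and stops movement when a later sound lands over 10 units from it.
; A debug key emits noise at the player; HandleSoundSense and PawnSensingFunctionTest are uncalled here.
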(event OnTargetPerceptionUpdated(AIPerception)
  (params (Actor :type Actor%20Object%20Reference) (Stimulus :type AI%20Stimulus%20Structure))
  (bind (_age _expirationage _strength _stimuluslocation) (Utilities|Struct|BreakAIStimulus Stimulus))
  (bind _returnvalue (AI|GetBlackboard 0))
  (bind _returnvalue_2 (Class|AIPerceptionSystem|GetSenseClassforStimulus Stimulus))
  (if (== _returnvalue_2 "/Script/AIModule.AISense_Hearing")
    (Utilities|FlowControl|Sequence
      (:then_0
        ;[1 1 1] Set Black Board(BB_SoundAI) Value / 블랙보드 값 설정
        (AI|Components|Blackboard|SetValueasFloat _returnvalue (Utilities|Name|MakeLiteralName "DistanceFromSound") (Math|Vector|Distance(Vector) _stimuluslocation (Transformation|GetActorLocation)))
        (AI|Components|Blackboard|SetValueasVector _returnvalue (Utilities|Name|MakeLiteralName "SoundLocation") _stimuluslocation)
        (AI|Components|Blackboard|SetValueasFloat _returnvalue (Utilities|Name|MakeLiteralName "Volume") _strength)
        (AI|Components|Blackboard|SetValueasBool _returnvalue (Utilities|Name|MakeLiteralName "DoesHeard") true))
      (:then_1
        ;[1 1 1] 소리로 Ai Move To 중에 새로운 소리가 들린다면 Movement Stop함
        (if (Utilities|Operators|EqualEqual "0,0.000000,0.000000" (Variables|Default|GetFirstSoundLocation) 0.01)
          (bind _output_get (Variables|Default|SetFirstSoundLocation _stimuluslocation))
          (else
            (bind _output_get_2 (Variables|Default|SetOhterSoundLocation _stimuluslocation))
            (if (> (Math|Vector|Distance(Vector) _output_get _output_get_2) 1e+01)
              (AI|Navigation|StopMovement (AI|GetAIController self))
              (Development|PrintString "멈춰")
              (Rendering|Debug|DrawDebugSphere _stimuluslocation 1e+02 12 "(R=0.000000,G=0.164614,B=1.000000,A=1.000000)" 3.0 1.0))))))))

(event EventBeginPlay
  (bind _returnvalue (AI|GetBlackboard 0))
  ;[1 1 1] Initialize default values in BlackBoard
  (AI|Components|Blackboard|SetValueasVector _returnvalue (Utilities|Name|MakeLiteralName "SoundLocation") (Transformation|GetActorLocation))
  (AI|Components|Blackboard|SetValueasObject _returnvalue (Utilities|Name|MakeLiteralName "SelfObject") self)
  (AI|Components|Blackboard|SetValueasVector _returnvalue (Utilities|Name|MakeLiteralName "SearchDirection") "0, 0, 0")
  (AI|Components|Blackboard|SetValueasBool _returnvalue (Utilities|Name|MakeLiteralName "DoesHeard") false))

(event Collision|EventActorBeginOverlap
  (params (OtherActor :type Actor%20Object%20Reference)))

(event EventTick
  (params (DeltaSeconds :type Float%20%28single-precision%29)))

(event Input|KeyboardEvents|DebugKey1
  (params (Key :type Key%20Structure :default "None") (ActionValue :type Input%20Action%20Value%20Structure))
  (bind _returnvalue (Game|Player|GetPlayerPawn 0))
  (:Pressed
    (Class|AISenseHearing|ReportNoiseEvent (Transformation|GetActorLocation _returnvalue) 3.0 _returnvalue 1e+04 "None")))

(fn ConstructionScript)

(fn HandleSoundSense
  (params (Stimulus :type AI%20Stimulus%20Structure%20%28by%20ref%29))
  (bind _returnvalue (AI|GetBlackboard 0))
  (bind (_age _expirationage _strength _stimuluslocation) (Utilities|Struct|BreakAIStimulus Stimulus))
  (bind _returnvalue_2 (Class|AIPerceptionSystem|GetSenseClassforStimulus Stimulus))
  (if (== _returnvalue_2 "/Script/AIModule.AISense_Hearing")
    ;[1 0.8431 0.3444] Set Black Board(BB_SoundAI) Value / 블랙보드 값 설정
    (AI|Components|Blackboard|SetValueasFloat _returnvalue (Utilities|Name|MakeLiteralName "DistanceFromSound") (Math|Vector|Distance(Vector) _stimuluslocation (Transformation|GetActorLocation)))
    (AI|Components|Blackboard|SetValueasVector _returnvalue (Utilities|Name|MakeLiteralName "SoundLocation") _stimuluslocation)
    (AI|Components|Blackboard|SetValueasFloat _returnvalue (Utilities|Name|MakeLiteralName "Volume") _strength)
    (AI|Components|Blackboard|SetValueasBool _returnvalue (Utilities|Name|MakeLiteralName "DoesHeard") true)
    (Rendering|Debug|DrawDebugSphere _stimuluslocation (* _strength 5e+01) 12 "(R=0.000000,G=0.164614,B=1.000000,A=1.000000)" 3.0 1.0)))

(fn PawnSensingFunctionTest
  (if (Actor|ActorHasTag "Player")
    (AI|Components|Blackboard|SetValueasBool (AI|GetBlackboard (AI|GetAIController self)) (Utilities|Name|MakeLiteralName "SeeingPlayer") true)))