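; BP_WorldDoor is a world door that swings open automatically away from the player when they approach, unless it is locked.
; Front and back overlap volumes set an open direction sign that multiplies a timeline-driven yaw on the door's relative rotation.
; A locked door only plays a sound, while an unlocked one plays an opening sound.
; The timeline reverses to close once the player has left both volumes.
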(event `self.FrontCheck.OnComponentBeginOverlap`
  (params (OverlappedComponent :type "PrimitiveComponent Object Reference") (OtherActor :type "Actor Object Reference") (OtherComp :type "PrimitiveComponent Object Reference") (OtherBodyIndex :type Integer) (bFromSweep :type Boolean) (SweepResult :type "HitResult Structure (by ref)"))
  (if (== OtherActor (`GameplayStatics.GetPlayerPawn` 0))
    (set `self.Front` true)
    (if (`self.DoorLock`)
      (`GameplayStatics.PlaySoundAtLocation` "/Game/World/Sound/DoorFX_06.DoorFX_06" (`self.K2_GetActorLocation`) (struct) 1.0 1.0 0.0 null null null null :!label _label)
      (elif (not (`self.IsDoorOpening`))
        (set `self.OpenDirection` 1.0)
        (set `self.IsDoorOpening` true :!label _label_2)
        (`GameplayStatics.PlaySoundAtLocation` "/Game/World/Sound/DoorFX_07.DoorFX_07" (`self.K2_GetActorLocation`) (struct) 1.0 1.0 0.0 null null null null)
        (`KismetSystemLibrary.PrintString` "Open")
        (bind (_direction _doorrotationz) (`Timeline|DoorTimelineComponent` :!label _label_3)
          (:`Update`
            (`SceneComponent.K2_SetRelativeRotation` (`self.Door`) (`KismetMathLibrary.MakeRotator` 0.0 0.0 (* _doorrotationz (`self.OpenDirection`))) false false)))))))

(event `self.BackCheck.OnComponentBeginOverlap`
  (params (OverlappedComponent :type "PrimitiveComponent Object Reference") (OtherActor :type "Actor Object Reference") (OtherComp :type "PrimitiveComponent Object Reference") (OtherBodyIndex :type Integer) (bFromSweep :type Boolean) (SweepResult :type "HitResult Structure (by ref)"))
  (if (== (`GameplayStatics.GetPlayerPawn` 0) OtherActor)
    (set `self.Back` true)
    (if (`self.DoorLock`)
      (goto _label)
      (elif (not (`self.IsDoorOpening`))
        (set `self.OpenDirection` -1.0)
        (goto _label_2)))))

(event `self.FrontCheck.OnComponentEndOverlap`
  (params (OverlappedComponent :type "PrimitiveComponent Object Reference") (OtherActor :type "Actor Object Reference") (OtherComp :type "PrimitiveComponent Object Reference") (OtherBodyIndex :type Integer))
  (if (== OtherActor (`GameplayStatics.GetPlayerPawn` 0))
    (set `self.Front` false)
    (if (not (`self.Back`))
      (set `self.IsDoorOpening` false :!label _label_4)
      (goto _label_3 :!via `Reverse`))))

(event `self.BackCheck.OnComponentEndOverlap`
  (params (OverlappedComponent :type "PrimitiveComponent Object Reference") (OtherActor :type "Actor Object Reference") (OtherComp :type "PrimitiveComponent Object Reference") (OtherBodyIndex :type Integer))
  (if (== OtherActor (`GameplayStatics.GetPlayerPawn` 0))
    (set `self.Back` false)
    (if (not (`self.Front`))
      (goto _label_4))))

(fn `UserConstructionScript`)