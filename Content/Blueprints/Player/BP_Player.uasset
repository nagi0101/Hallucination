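; First-person player character with crouch, sprint, hold-breath, physics object grabbing and temporary grow or shrink skills.
; Enhanced Input events drive the actions; grabbing, marked unfinished, line-traces from the camera and holds the hit component ahead through a PhysicsHandle.
; Tick updates the grab target, velocity-based camera shake, stamina and post-process parameters, calling functions defined outside these graphs.
; The mutually exclusive size skills rescale the actor, then restore it after a delay.
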(event `GetBigger`
  ;[1 1 1] Skill
  (if (and (not (`self.IsBigger`)) (not (`self.IsSmaller`)))
    (set `self.IsBigger` true)
    (`self.SetActorScale3D` (2.0 2.0 2.0))
    (`KismetSystemLibrary.Delay` (`self.MaintainedTimeToBigger`))
    (`self.SetActorScale3D` (1.0 1.0 1.0))
    (set `self.IsBigger` false)))

(event `GetSmaller`
  ;[1 1 1] Skill
  (if (and (not (`self.IsBigger`)) (not (`self.IsSmaller`)))
    (set `self.IsSmaller` true)
    (`self.SetActorScale3D` (0.5 0.5 0.5))
    (`KismetSystemLibrary.Delay` (`self.MaintainedTimeToSmaller`))
    (`self.SetActorScale3D` (1.0 1.0 1.0))
    (set `self.IsSmaller` false)))

(event `self.ReceiveBeginPlay`
  ;[1 1 1] Enhanced Input Setting
  (bind _asbp_player_controller (cast `/Game/Blueprints/Player/BP_PlayerController` (`self.GetController`)))
  (`EnhancedInputSubsystemInterface.AddMappingContext` (pcsubsystem `EnhancedInputLocalPlayerSubsystem` _asbp_player_controller) "/Game/Blueprints/Player/Inputs/IMC_Player.IMC_Player" 0 (struct)))

(event `EnhancedInput|/Game/Blueprints/Player/Inputs/IA_Pickup`
  (params (ActionValue :type Boolean) (ElapsedSeconds :type "Float (double-precision)") (TriggeredSeconds :type "Float (double-precision)") (InputAction :type "InputAction Object Reference" :default "/Game/Blueprints/Player/Inputs/IA_Pickup.IA_Pickup"))
  (bind _firstpersoncamera (`self.FirstPersonCamera`))
  (bind _returnvalue (`SceneComponent.K2_GetComponentLocation` _firstpersoncamera))
  ;[1 1 1] Grab and Move Object(미완) - F key
  (:`Triggered`
    (bind (_outhit _returnvalue_2) (`KismetSystemLibrary.LineTraceSingle` _returnvalue (+ _returnvalue (* (`KismetMathLibrary.GetForwardVector` (`SceneComponent.K2_GetComponentRotation` _firstpersoncamera)) 500.0)) "TraceTypeQuery1"))
    (if _returnvalue_2
      (bind (_bblockinghit _binitialoverlap _time _distance _location _impactpoint _normal _impactnormal _physmat _hitactor _hitcomponent) (`GameplayStatics.BreakHitResult` _outhit))
      (`PrimitiveComponent.WakeRigidBody` _hitcomponent "None")
      (`PhysicsHandleComponent.GrabComponentAtLocation` (`self.PhysicsHandle`) _hitcomponent "None" (`SceneComponent.K2_GetComponentLocation` _hitcomponent))
      (set `self.IsGrabbing` true)))
  (:`Completed`
    (if (`self.IsGrabbing`)
      (`PhysicsHandleComponent.ReleaseComponent` (`self.PhysicsHandle`))
      (set `self.IsGrabbing` false))))

(event `self.ReceiveTick`
  (params (DeltaSeconds :type "Float (single-precision)"))
  (bind _firstpersoncamera (`self.FirstPersonCamera`))
  (`|ExecutionSequence`
    (:`then_0`
      ;[1 1 1] Grab and Move Object(미완) - F key
      (if (`self.IsGrabbing`)
        (`PhysicsHandleComponent.SetTargetLocation` (`self.PhysicsHandle`) (+ (`SceneComponent.K2_GetComponentLocation` _firstpersoncamera) (* (`KismetMathLibrary.GetForwardVector` (`SceneComponent.K2_GetComponentRotation` _firstpersoncamera)) 500.0)))))
    (:`then_1`
      ;[1 1 1] Camera Shaking
      (`self.ShakeCamera`))
    (:`then_2`
      (`self.CheckStemina` (`GameplayStatics.GetWorldDeltaSeconds`)))
    (:`then_3`
      (`self.SetPostProcessParameter`))))

(event `ShakeCamera`
  ;[1 1 1] Camera Shaking
  (`self.SetCameraShake` (`self.GetVelocity`)))

(event `EnhancedInput|/Game/Blueprints/Player/Inputs/IA_Run`
  (params (ActionValue :type Boolean) (ElapsedSeconds :type "Float (double-precision)") (TriggeredSeconds :type "Float (double-precision)") (InputAction :type "InputAction Object Reference" :default "/Game/Blueprints/Player/Inputs/IA_Run.IA_Run"))
  ;[1 1 1] Sprint
  (:`Started`
    (`self.StartSprint`))
  (:`Completed`
    (`self.EndSprint`)))

(event `EnhancedInput|/Game/Blueprints/Player/Inputs/IA_Crouch`
  (params (ActionValue :type Boolean) (ElapsedSeconds :type "Float (double-precision)") (TriggeredSeconds :type "Float (double-precision)") (InputAction :type "InputAction Object Reference" :default "/Game/Blueprints/Player/Inputs/IA_Crouch.IA_Crouch"))
  ;[1 1 1] Crouch
  (:`Triggered`
    (`self.Crouch`))
  (:`Completed`
    (`self.UnCrouch`)))

(event `EnhancedInput|/Game/Blueprints/Player/Inputs/IA_HoldBreath`
  (params (ActionValue :type Boolean) (ElapsedSeconds :type "Float (double-precision)") (TriggeredSeconds :type "Float (double-precision)") (InputAction :type "InputAction Object Reference" :default "/Game/Blueprints/Player/Inputs/IA_HoldBreath.IA_HoldBreath"))
  ;[1 1 1] Hold Breath
  (:`Started`
    (`self.StartHoldBreath`))
  (:`Completed`
    (`self.EndHoldBreath`)))

(fn `UserConstructionScript`)